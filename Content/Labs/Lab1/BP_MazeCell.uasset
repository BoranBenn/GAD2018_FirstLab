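; BP_MazeCell is a maze tile actor that builds its geometry in the construction script; its event graph is inactive.
; GridSize sets wall length and thickness, and SizeCubeScale turns dimensions into mesh scales for the floor and added pieces.
; West, South, East and North flags each add a wall mesh along their edge.
; The NorthWall branch also adds an overhead slab at WallHeight and a downward-facing spotlight.
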(fn `UserConstructionScript`
  (locals (WallThickness :type "Float (double-precision)") (WallLength :type "Float (double-precision)"))
  (bind _gridsize (`self.GridSize`))
  (bind _walllength (`local.WallLength`))
  (bind _returnvalue (* (`self.WallHeight`) 0.5))
  (set `local.WallLength` _gridsize)
  (set `local.WallThickness` (* _gridsize 0.1))
  (`SceneComponent.SetRelativeScale3D` (`self.Floor`) (`self.SizeCubeScale` (`KismetMathLibrary.MakeVector` _walllength _walllength (`local.WallThickness`))))
  (if (`self.WestWall`)
    (`AddComponent|NODE_AddStaticMeshComponent-0` :`RelativeTransform` (`KismetMathLibrary.MakeTransform` (0.0 0.0 0.0) (struct) (`self.SizeCubeScale` (`KismetMathLibrary.MakeVector` (`local.WallLength`) (`local.WallThickness`) (`self.WallHeight`))))))
  (if (`self.SouthWall`)
    (`AddComponent|NODE_AddStaticMeshComponent-1` :`RelativeTransform` (`KismetMathLibrary.MakeTransform` (0.0 0.0 0.0) (struct) (`self.SizeCubeScale` (`KismetMathLibrary.MakeVector` (`local.WallThickness`) (`local.WallLength`) (`self.WallHeight`))))))
  (if (`self.EastWall`)
    (`AddComponent|NODE_AddStaticMeshComponent-2` :`RelativeTransform` (`KismetMathLibrary.MakeTransform` (`KismetMathLibrary.MakeVector` 0.0 (- (`local.WallLength`) (`local.WallThickness`))) (struct) (`self.SizeCubeScale` (`KismetMathLibrary.MakeVector` (`local.WallLength`) (`local.WallThickness`) (`self.WallHeight`))))))
  (if (`self.NorthWall`)
    (`AddComponent|NODE_AddStaticMeshComponent-3` :`RelativeTransform` (`KismetMathLibrary.MakeTransform` (`KismetMathLibrary.MakeVector` (- (`local.WallLength`) (`local.WallThickness`))) (struct) (`self.SizeCubeScale` (`KismetMathLibrary.MakeVector` (`local.WallThickness`) (`local.WallLength`) (`self.WallHeight`)))))
    (`AddComponent|NODE_AddStaticMeshComponent-4` :`RelativeTransform` (`KismetMathLibrary.MakeTransform` (`KismetMathLibrary.MakeVector` 0.0 0.0 (`self.WallHeight`)) (struct) (`self.SizeCubeScale` (`KismetMathLibrary.MakeVector` (`local.WallLength`) (`self.WallHeight`) (`local.WallThickness`)))))
    (`AddComponent|NODE_AddSpotLightComponent-0` :`RelativeTransform` (`KismetMathLibrary.MakeTransform` (`KismetMathLibrary.MakeVector` _returnvalue _returnvalue (`self.WallHeight`)) (struct :`Pitch` -90.0)))))